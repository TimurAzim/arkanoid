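; Player pawn that launches balls from its Arrow component and tracks the player's lives in a ball game.
; SpawnBall spawns one main BP_Ball while lives remain and none is alive, binding its destruction to decrement lives and print "Game over!" at zero.
; When the Cube overlaps a BP_Bonus, it destroys the bonus and spawns a half-size extra ball, which is not bound to life loss.
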(event OnComponentBeginOverlap(Cube)
  (params (OverlappedComponent :type Primitive%20Component%20Object%20Reference) (OtherActor :type Actor%20Object%20Reference) (OtherComp :type Primitive%20Component%20Object%20Reference) (OtherBodyIndex :type Integer) (bFromSweep :type Boolean) (SweepResult :type Hit%20Result%20Structure%20%28by%20ref%29))
  (bind _asbp_bonus (Utilities|Casting|CastToBP_Bonus OtherActor))
  (CallFunction|BallEvent)
  (Actor|DestroyActor _asbp_bonus))

(event Custom|SpawnBall
  (if (not (<= (Variables|Default|GetPlayerLives) 0))
    (Variables|Default|GetAliveBall
      (:then)
      (:else
        (bind _returnvalue (Game|SpawnActorfromClass "/Game/MyGame/Blueprint/BP_Ball.BP_Ball_C" (Math|Transform|MakeTransform (Transformation|GetWorldLocation (Variables|Default|GetArrow))) "Undefined" 0 0))
        (bind _output_get (Variables|Default|SetAliveBall _returnvalue))
        (Game|BindEventtoOnDestroyed _output_get (delegate Custom|BallisDed))))))

(event Custom|BallisDed
  (params (DestroyedActor :type Actor%20Object%20Reference))
  (bind _result (Math|Integer|DecrementInt (Variables|Default|GetPlayerLives))
    (:%20%20
      (if (<= _result 0)
        (Development|PrintString "Game over!")))))

(event Custom|BallEvent
  (Game|SpawnActorfromClass "/Game/MyGame/Blueprint/BP_Ball.BP_Ball_C" (Math|Transform|MakeTransform (Transformation|GetWorldLocation (Variables|Default|GetArrow)) "0, 0, 0" "0.500000,0.500000,0.500000") "Undefined" 0 0))

(event Collision|EventActorBeginOverlap
  (params (OtherActor :type Actor%20Object%20Reference)))

(event EventTick
  (params (DeltaSeconds :type Float%20%28single-precision%29)))

(fn ConstructionScript)