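; BP_MyPlayerControler is a player controller that slides a possessed BP_MyPown pawn sideways and spawns balls on input.
; BeginPlay sets game-only input mode, and possession caches the pawn as BP_MyPown.
; The LeftRight axis moves the pawn along Y with a swept, delta-time-scaled offset.
; The SpawnBall action forwards to the pawn's own SpawnBall function.
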(event EventPossess
  (params (PossessedPawn :type Pawn%20Object%20Reference))
  (bind _asbp_my_pown (Utilities|Casting|CastToBP_MyPown PossessedPawn))
  (Variables|Default|SetMy%20Pown _asbp_my_pown))

(event EventBeginPlay
  (Input|SetInputModeGameOnly self))

(event Input|ActionEvents|InputActionSpawnBall
  (params (Key :type Key%20Structure :default "None"))
  (:Pressed
    (Default|SpawnBall (Variables|Default|GetMy%20Pown))))

(event Input|AxisEvents|InputAxisLeftRight
  (params (AxisValue :type Float%20%28single-precision%29))
  (Transformation|AddActorWorldOffset (Variables|Default|GetMy%20Pown) (Math|Vector|MakeVector 0.0 (* AxisValue (Utilities|Time|GetWorldDeltaSeconds) (Variables|Default|GetSpeed)) 0.0) true))

(fn ConstructionScript)