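; BP_Ball is a ball actor that travels in a straight line and bounces off blocking surfaces.
; Each Tick it moves by Direction, Speed and delta time using a swept world offset, applied on X and Y only.
; On a blocking hit it reflects Direction about the hit normal and raises Speed by AddSpeed up to a fixed cap.
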(event EventTick
  (params (DeltaSeconds :type Float%20%28single-precision%29))
  (bind _sweephitresult (Transformation|AddActorWorldOffset (Math|Vector|MakeVector (.x (* (Variables|Default|GetDirection) (* (Variables|Default|GetSpeed) DeltaSeconds))) (.y (* (Variables|Default|GetDirection) (* (Variables|Default|GetSpeed) DeltaSeconds))) 0.0) true))
  (if (.bBlockingHit (Collision|BreakHitResult _sweephitresult))
    (Variables|Default|SetDirection (Math|Vector|GetReflectionVector (Variables|Default|GetDirection) (.Normal (Collision|BreakHitResult _sweephitresult))))
    (Variables|Default|SetSpeed (Math|Float|Min(Float) (+ (Variables|Default|GetSpeed) (Variables|Default|GetAddSpeed)) 1.5e+03))))

(fn ConstructionScript)