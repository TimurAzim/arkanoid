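; BP_Cubes_Generated lays out a padded X by Y grid of BP_Child_Block actors at its location when play begins.
; The construction script previews the grid in the editor with static mesh components, which BeginPlay destroys before spawning the real blocks.
; Spawned blocks are stored in CubseArrey, whose length GetCubesForWin returns, presumably as a win-condition count.
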(event EventBeginPlay
  (bind _returnvalue (Transformation|GetActorLocation))
  (for _array_element (Variables|Default|GetPreviewArrey)
    (Components|DestroyComponent _array_element))
  (for _index (range 0 (Variables|Default|GetX))
    (for _index_2 (range 0 (Variables|Default|GetY))
      (bind _returnvalue_2 (Game|SpawnActorfromClass "/Game/MyGame/Blueprint/BP_Child_Block.BP_Child_Block_C" (Math|Transform|MakeTransform (Math|Vector|MakeVector (+ (Math|Conversions|ToFloat(Integer) (* _index (Variables|Default|GetPadding))) (.x _returnvalue)) (+ (.y _returnvalue) (Math|Conversions|ToFloat(Integer) (* _index_2 (Variables|Default|GetPadding)))) (.z _returnvalue))) "Undefined" 0 0))
      (Utilities|Array|Add (Variables|Default|GetCubseArrey) _returnvalue_2))))

(fn ConstructionScript
  (for _index (range 0 (Variables|Default|GetX))
    (for _index_2 (range 0 (Variables|Default|GetY))
      (bind _returnvalue (AddComponent|AddStaticMeshComponent false (Math|Transform|MakeTransform (Math|Vector|MakeVector (Math|Conversions|ToFloat(Integer) (* _index (Variables|Default|GetPadding))) (Math|Conversions|ToFloat(Integer) (* _index_2 (Variables|Default|GetPadding))) 0.0))))
      (Utilities|Array|Add (Variables|Default|GetPreviewArrey) _returnvalue))))

(fn GetCubesforWin
  (return (Utilities|Array|Length (Variables|Default|GetCubseArrey))))