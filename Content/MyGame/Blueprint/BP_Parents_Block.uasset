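; BP_Parents_Block is a breakable block, apparently a base class, that takes damage from BP_Ball hits.
; The construction script gives it two lives; each ball hit removes one, swapping the cube to a red material while lives remain and destroying the actor at zero.
; On BeginPlay, a coin flip decides whether its OnDestroyed event is bound to spawn a BP_Bonus at the block's location.
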(event Custom|BallHit
  (bind _result (Math|Integer|DecrementInt (Variables|Default|GetLive))
    (:%20%20
      (if (<= _result 0)
        (Actor|DestroyActor)
        (else
          (Rendering|Material|SetMaterial (Variables|Default|GetCube) 0 "/Engine/EngineDebugMaterials/VertexColorViewMode_RedOnly.VertexColorViewMode_RedOnly"))))))

(event Custom|SpawnBonuse
  (params (DestroyedActor :type Actor%20Object%20Reference))
  (Game|SpawnActorfromClass "/Game/MyGame/Blueprint/Bonus/BP_Bonus.BP_Bonus_C" (Math|Transform|MakeTransform (Transformation|GetActorLocation)) "AlwaysSpawn" 0 0))

(event Collision|EventHit
  (params (MyComp :type Primitive%20Component%20Object%20Reference) (Other :type Actor%20Object%20Reference) (OtherComp :type Primitive%20Component%20Object%20Reference) (bSelfMoved :type Boolean) (HitLocation :type Vector :default "0, 0, 0") (HitNormal :type Vector :default "0, 0, 0") (NormalImpulse :type Vector :default "0, 0, 0") (Hit :type Hit%20Result%20Structure%20%28by%20ref%29))
  (Utilities|Casting|CastToBP_Ball Other)
  (CallFunction|BallHit))

(event EventBeginPlay
  (if (Math|Random|RandomBoolwithWeight 0.5)
    (Game|BindEventtoOnDestroyed (delegate Custom|SpawnBonuse))))

(fn ConstructionScript
  (Variables|Default|SetLive 2))